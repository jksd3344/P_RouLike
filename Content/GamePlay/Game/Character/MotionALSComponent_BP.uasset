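; Advanced Locomotion System (ALS) style component that tracks motion state for its owning BP_RouLikeCharacter.
; Each Tick derives acceleration, speed, movement input and aim yaw rate from the cached owner, keeping last movement rotations.
; When MovementState is None, it also resolves allowed gait from stance, rotation mode and desired gait.
; Getters expose these values and states; a CanSprint check exists but is not wired into gait selection.
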(event `self.ReceiveTick`
  (params (DeltaSeconds :type "Float (single-precision)"))
  (`|ExecutionSequence`
    (:`then_0`
      (`self.Set Essential Values`)
      (switch `/Game/AdvancedLocomotionV4/Data/Enums/ALS_MovementState` (`self.MovementState`)
        (:`NewEnumerator0`
          (`self.Update Character Movement`))))))

(fn `AlsGetEssentialValue`
  (returns (Velocity :type "Vector Structure") (Acceleration :type "Vector Structure") (Movement :type "Vector Structure") (IsMoving :type Boolean) (HasMovementInput :type Boolean) (Speed :type "Float (single-precision)") (MovementInputAmout :type "Float (single-precision)") (AimingRotation :type "Rotator Structure") (AimYawRate :type "Float (single-precision)"))
  (bind _asbp_rou_like_character (`self.GetCharacterBP`))
  (return (`Actor.GetVelocity` _asbp_rou_like_character) (`self.Acceleration`) (`CharacterMovementComponent.GetCurrentAcceleration` (`Character.CharacterMovement` _asbp_rou_like_character)) (`self.IsMoving`) (`self.HasMovementInput`) (`self.Speed`) (`self.MovementInputAmount`) (`Pawn.GetControlRotation` _asbp_rou_like_character) (`self.AimYawRate`)))

(fn `BPI_Get_CurrentStates`
  (returns (PawnMovementMode :type "EMovementMode Enum") (MovementState :type "/Game/AdvancedLocomotionV4/Data/Enums/ALS_MovementState Enum") (PrevMovementState :type "/Game/AdvancedLocomotionV4/Data/Enums/ALS_MovementState Enum") (MovementAction :type "/Game/AdvancedLocomotionV4/Data/Enums/ALS_MovementAction Enum") (RotationMode :type "/Game/AdvancedLocomotionV4/Data/Enums/ALS_RotationMode Enum") (ActualGait :type "/Game/AdvancedLocomotionV4/Data/Enums/ALS_Gait Enum") (ActualStance :type "/Game/AdvancedLocomotionV4/Data/Enums/ALS_Stance Enum") (ViewMode :type "/Game/AdvancedLocomotionV4/Data/Enums/ALS_ViewMode Enum") (OverlayState :type "/Game/AdvancedLocomotionV4/Data/Enums/ALS_OverlayState Enum"))
  (return (`CharacterMovementComponent.MovementMode` (`Character.CharacterMovement` (`self.GetCharacterBP`))) (`self.MovementState`) (`self.PrevMovementState`) (`self.MovementAction`) (`self.RotationMode`) (`self.Gait`) (`self.Stance`) (`self.ViewMode`) (`self.OverlayState`)))

(fn `Calculate Relative Acceleration`
  (returns (ReturnValue :type "Vector Structure"))
  (bind _charactermovement (`Character.CharacterMovement` (`self.GetCharacterBP`)))
  (bind _returnvalue (`CharacterMovementComponent.GetMaxAcceleration` _charactermovement))
  (bind _returnvalue_2 (`CharacterMovementComponent.GetMaxBrakingDeceleration` _charactermovement))
  (if (> (`KismetMathLibrary.Dot_VectorVector` (`self.Acceleration`) (`self.CharacterOldVeloci`)) 0.0)
    (return (`KismetMathLibrary.LessLess_VectorRotator` (/ (`KismetMathLibrary.Vector_ClampSizeMax` (`self.Acceleration`) _returnvalue) _returnvalue) (`Actor.K2_GetActorRotation` (`self.GetCharacterBP`))))
    (else
      (return (`KismetMathLibrary.LessLess_VectorRotator` (/ (`KismetMathLibrary.Vector_ClampSizeMax` (`self.Acceleration`) _returnvalue_2) _returnvalue_2) (`Actor.K2_GetActorRotation` (`self.GetCharacterBP`)))))))

(fn `CanSprint`
  (returns (NewParam :type Boolean))
  (bind _asbp_rou_like_character (`self.GetCharacterBP`))
  (bind (_returnvalue_roll _returnvalue_pitch _returnvalue_yaw) (`KismetMathLibrary.BreakRotator` (`KismetMathLibrary.NormalizedDeltaRotator` (`KismetMathLibrary.Conv_VectorToRotator` (`CharacterMovementComponent.GetCurrentAcceleration` (`Character.CharacterMovement` _asbp_rou_like_character))) (`Pawn.GetControlRotation` _asbp_rou_like_character))))
  ;[1 1 1] 根据旋转模式和当前加速度（输入）旋转来确定角色当前是否能够冲刺。如果角色处于“注视旋转”模式，则只有在有完整的移动输入并且相对于相机向前+或-50度的情况下才允许冲刺。
  (if (`self.HasMovementInput`)
    (switch `/Game/AdvancedLocomotionV4/Data/Enums/ALS_RotationMode` (`self.RotationMode`)
      (:`NewEnumerator0`
        (return (> (`self.MovementInputAmount`) 0.9)))
      (:`NewEnumerator1`
        (return (and (> (`self.MovementInputAmount`) 0.9) (< (`KismetMathLibrary.Abs` _returnvalue_yaw) 50.0))))
      (:`NewEnumerator3`
        (return false)))
    (else
      (return false))))

(fn `Get Allowed Gait`
  (returns (DesiredGait :type "/Game/GamePlay/Game/Animation/AnimAssert/Data/Enums/ALS_Gait_RL Enum"))
  (switch `/Game/AdvancedLocomotionV4/Data/Enums/ALS_Stance` (`self.Stance`)
    (:`NewEnumerator0`
      (switch `/Game/AdvancedLocomotionV4/Data/Enums/ALS_RotationMode` (`self.RotationMode`)
        (:`NewEnumerator0`
          _)
        (:`NewEnumerator1`
          _))
      (switch `/Game/GamePlay/Game/Animation/AnimAssert/Data/Enums/ALS_Gait_RL` (`self.DesiredGait`)
        (:`NewEnumerator0`
          (return "NewEnumerator0"))
        (:`NewEnumerator1`
          (return "NewEnumerator1"))))
    (:`NewEnumerator1`
      (switch `/Game/GamePlay/Game/Animation/AnimAssert/Data/Enums/ALS_Gait_RL` (`self.DesiredGait`)
        (:`NewEnumerator0`
          (return "NewEnumerator0"))
        (:`NewEnumerator1`
          _)
        (:`NewEnumerator2`
          _))
      (return "NewEnumerator1"))))

(fn `GetCharacterBP`
  (returns (`AsBP Rou Like Character` :type "/Game/GamePlay/Game/Character/BP_RouLikeCharacter Object Reference"))
  (bind _as_bp_rou_like_character (`self.As BP Rou Like Character`))
  (`/Engine/EditorBlueprintResources/StandardMacros.IsValid` _as_bp_rou_like_character
    (:`Is Valid`
      (return _as_bp_rou_like_character))
    (:`Is Not Valid`
      (bind _asbp_rou_like_character (cast `/Game/GamePlay/Game/Character/BP_RouLikeCharacter` (`self.GetOwner`)))
      (`/Engine/EditorBlueprintResources/StandardMacros.IsValid` _asbp_rou_like_character
        (:`Is Valid`
          (bind _output_get (set `self.As BP Rou Like Character` _asbp_rou_like_character))
          (return _output_get))))))

(fn `Set Essential Values`
  (bind _asbp_rou_like_character (`self.GetCharacterBP`))
  (bind _returnvalue (`Actor.GetVelocity` (`self.GetCharacterBP`)))
  (bind (_returnvalue_x _returnvalue_y) (`KismetMathLibrary.BreakVector` (`Actor.GetVelocity` _asbp_rou_like_character)))
  (bind (_returnvalue_roll _returnvalue_pitch _returnvalue_yaw) (`KismetMathLibrary.BreakRotator` (`Pawn.GetControlRotation` (`self.GetCharacterBP`))))
  (bind _charactermovement (`Character.CharacterMovement` _asbp_rou_like_character))
  (`|ExecutionSequence`
    (:`then_0`
      ;[1 1 1] 角色加速度/角色倾斜偏移
      (set `self.Acceleration` (/ (- _returnvalue (`self.CharacterOldVeloci`)) (`GameplayStatics.GetWorldDeltaSeconds`)))
      (set `self.CharacterOldVeloci` _returnvalue)
      (set `self.RelativeAccelerationAmount` (`self.Calculate Relative Acceleration`)))
    (:`then_1`
      ;[1 1 1] 通过获取角色的速度来确定角色是否在移动。“速度”等于水平（x y）速度的长度，因此不考虑垂直移动 / 如果角色正在移动，请更新最后一个速度旋转。之所以保存此值，是因为即使在角色停止后，也可以知道移动的最后方向。
      (bind _output_get (set `self.Speed` (`KismetMathLibrary.VSize` (`KismetMathLibrary.MakeVector` _returnvalue_x _returnvalue_y))))
      (bind _output_get_2 (set `self.IsMoving` (> _output_get 0.0)))
      (if _output_get_2
        (set `self.LastVelocityRotation` (`KismetMathLibrary.Conv_VectorToRotator` (`Actor.GetVelocity` (`self.GetCharacterBP`))))))
    (:`then_2`
      ;[1 1 1] 通过获取角色的移动输入量来确定角色是否有移动输入。移动输入量等于当前加速度除以最大加速度，因此其范围为0-1，1是最大可能的输入量，0是零。如果角色有移动输入，请更新“最后一次移动输入旋转”。
      (bind _output_get_3 (set `self.MovementInputAmount` (/ (`KismetMathLibrary.VSize` (`CharacterMovementComponent.GetCurrentAcceleration` _charactermovement)) (`CharacterMovementComponent.GetMaxAcceleration` _charactermovement))))
      (bind _output_get_4 (set `self.HasMovementInput` (> _output_get_3 0.0)))
      (if _output_get_4
        (set `self.LastMovementInputRotation` (`KismetMathLibrary.Conv_VectorToRotator` (`CharacterMovementComponent.GetCurrentAcceleration` (`Character.CharacterMovement` (`self.GetCharacterBP`)))))))
    (:`then_3`
      ;[1 1 1] 通过比较当前和以前的目标偏航值除以增量秒来设置目标偏航率。这表示相机从左向右旋转的速度。
      (set `self.AimYawRate` (/ (- _returnvalue_yaw (`self.PreviousAimYaw`)) (`GameplayStatics.GetWorldDeltaSeconds`))))))

(fn `Update Character Movement`
  (`|ExecutionSequence`
    (:`then_0`
      ;[1 1 1] Set the Allowed Gait
      (set `self.AllowedGait` (`self.Get Allowed Gait`)))))