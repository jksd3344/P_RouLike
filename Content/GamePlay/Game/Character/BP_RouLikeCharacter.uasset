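; Roguelike player character that maps input to an ALS-style motion component for gait, stance, rotation mode and ragdoll.
; Walk toggles walk/run and sprint is held while grounded, both routed through Server/Multi-named custom events.
; A retriggerable-delay press-counter macro limits stance toggling to the first press, with multi-press unused and roll logic unconnected.
; Movement mode and crouch callbacks are forwarded to the component to keep its state in sync.
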(event `InputAction|WalkAction`
  (params (Key :type "Key Structure"))
  ;[1 1 1] 步态动作类型1：按“行走动作”切换行走/跑步，按住“冲刺动作”进行冲刺。
  (:`Pressed`
    (`self.WalkActionMove`)))

(event `WalkActionMove`
  ;[1 1 1] 步态动作类型1：按“行走动作”切换行走/跑步，按住“冲刺动作”进行冲刺。
  (`self.WalkActionMoveMulti`))

(event `WalkActionMoveMulti`
  (bind _motionalscomponent_bp (`self.MotionALSComponent_BP`))
  ;[1 1 1] 步态动作类型1：按“行走动作”切换行走/跑步，按住“冲刺动作”进行冲刺。
  (switch `/Game/GamePlay/Game/Animation/Data/Enums/ALS_Gait_RL` (`/Game/GamePlay/Game/Character/MotionALSComponent_BP.DesiredGait` _motionalscomponent_bp)
    (:`NewEnumerator0`
      (set `/Game/GamePlay/Game/Character/MotionALSComponent_BP.DesiredGait` "NewEnumerator1" _motionalscomponent_bp))
    (:`NewEnumerator1`
      (set `/Game/GamePlay/Game/Character/MotionALSComponent_BP.DesiredGait` "NewEnumerator0" _motionalscomponent_bp))))

(event `SpringActionServer`
  (params (DesiredGait :type "/Game/GamePlay/Game/Animation/Data/Enums/ALS_Gait_RL Enum" :default "NewEnumerator0"))
  ;[1 1 1] 步态动作类型1：按“行走动作”切换行走/跑步，按住“冲刺动作”进行冲刺。
  (switch `/Game/GamePlay/Game/Animation/Data/Enums/ALS_MovementState_RL` (`/Game/GamePlay/Game/Character/MotionALSComponent_BP.MovementState` (`self.MotionALSComponent_BP`))
    (:`NewEnumerator1`
      (`self.SpringActionMulti` DesiredGait))))

(event `SpringActionMulti`
  (params (DesiredGait :type "/Game/GamePlay/Game/Animation/Data/Enums/ALS_Gait_RL Enum" :default "NewEnumerator0"))
  ;[1 1 1] 步态动作类型1：按“行走动作”切换行走/跑步，按住“冲刺动作”进行冲刺。
  (set `/Game/GamePlay/Game/Character/MotionALSComponent_BP.DesiredGait` DesiredGait (`self.MotionALSComponent_BP`)))

(event `InputAction|Spring`
  (params (Key :type "Key Structure"))
  ;[1 1 1] 步态动作类型1：按“行走动作”切换行走/跑步，按住“冲刺动作”进行冲刺。
  (:`Pressed`
    (`self.SpringActionServer` "NewEnumerator2"))
  (:`Released`
    (`self.SpringActionServer` "NewEnumerator1")))

(event `InputAction|StanceAction`
  (params (Key :type "Key Structure"))
  (bind _motionalscomponent_bp (`self.MotionALSComponent_BP`))
  ;[1 1 1] 注释
  (:`Pressed`
    (switch `/Game/GamePlay/Game/Animation/Data/Enums/ALS_MovementAction_RL` (`/Game/GamePlay/Game/Character/MotionALSComponent_BP.MovementAction` _motionalscomponent_bp)
      (:`NewEnumerator4`
        (`self.新建宏` 0.3
          (:`First Press`
            (switch `/Game/GamePlay/Game/Animation/Data/Enums/ALS_MovementState_RL` (`/Game/GamePlay/Game/Character/MotionALSComponent_BP.MovementState` _motionalscomponent_bp)
              (:`NewEnumerator1`
                (switch `/Game/GamePlay/Game/Animation/Data/Enums/ALS_Stance_RL` (`/Game/GamePlay/Game/Character/MotionALSComponent_BP.Stance` (`self.MotionALSComponent_BP`))
                  (:`NewEnumerator0`
                    (set `/Game/GamePlay/Game/Character/MotionALSComponent_BP.DesiredStance` "NewEnumerator1" (`self.MotionALSComponent_BP`))
                    (`self.Crouch`))
                  (:`NewEnumerator1`
                    (set `/Game/GamePlay/Game/Character/MotionALSComponent_BP.DesiredStance` "NewEnumerator0" (`self.MotionALSComponent_BP`))
                    (`self.UnCrouch`)))))))))))

(event `self.K2_OnMovementModeChanged`
  (params (PrevMovementMode :type "EMovementMode Enum" :default "MOVE_None") (NewMovementMode :type "EMovementMode Enum" :default "MOVE_None") (PrevCustomMode :type Byte) (NewCustomMode :type Byte))
  ;[1 1 1] 注释
  (`parent.K2_OnMovementModeChanged` PrevMovementMode NewMovementMode PrevCustomMode NewCustomMode)
  (`/Game/GamePlay/Game/Character/MotionALSComponent_BP.On Character Movement Mode Changed` (`self.MotionALSComponent_BP`) PrevMovementMode NewMovementMode PrevCustomMode NewCustomMode))

(event `self.K2_OnStartCrouch`
  (params (HalfHeightAdjust :type "Float (single-precision)") (ScaledHalfHeightAdjust :type "Float (single-precision)"))
  ;[1 1 1] 注释
  (`parent.K2_OnStartCrouch` HalfHeightAdjust ScaledHalfHeightAdjust)
  (`/Game/GamePlay/Game/Character/MotionALSComponent_BP.On Stance Changed` (`self.MotionALSComponent_BP`) "NewEnumerator1"))

(event `self.K2_OnEndCrouch`
  (params (HalfHeightAdjust :type "Float (single-precision)") (ScaledHalfHeightAdjust :type "Float (single-precision)"))
  ;[1 1 1] 注释
  (`parent.K2_OnEndCrouch` HalfHeightAdjust ScaledHalfHeightAdjust)
  (`/Game/GamePlay/Game/Character/MotionALSComponent_BP.On Stance Changed` (`self.MotionALSComponent_BP`) "NewEnumerator0"))

(event `InputAction|SelectRotationMode_1`
  (params (Key :type "Key Structure"))
  (bind _motionalscomponent_bp (`self.MotionALSComponent_BP`))
  ;[1 1 1] 注释
  (:`Pressed`
    (bind _output_get (set `/Game/GamePlay/Game/Character/MotionALSComponent_BP.DesiredRotationMode` "NewEnumerator0" _motionalscomponent_bp))
    (`/Game/GamePlay/Game/Character/MotionALSComponent_BP.BPI_Set_RotationMode` _motionalscomponent_bp _output_get)))

(event `InputAction|SelectRotationMode_2`
  (params (Key :type "Key Structure"))
  (bind _motionalscomponent_bp (`self.MotionALSComponent_BP`))
  ;[1 1 1] 注释
  (:`Pressed`
    (bind _output_get (set `/Game/GamePlay/Game/Character/MotionALSComponent_BP.DesiredRotationMode` "NewEnumerator1" _motionalscomponent_bp))
    (`/Game/GamePlay/Game/Character/MotionALSComponent_BP.BPI_Set_RotationMode` _motionalscomponent_bp _output_get)))

(event `InputAction|RagdollAction`
  (params (Key :type "Key Structure"))
  (bind _motionalscomponent_bp (`self.MotionALSComponent_BP`))
  ;[1 1 1] 注释
  (:`Pressed`
    (switch `/Game/GamePlay/Game/Animation/Data/Enums/ALS_MovementState_RL` (`/Game/GamePlay/Game/Character/MotionALSComponent_BP.MovementState` (`self.MotionALSComponent_BP`))
      (:`NewEnumerator0`
        (`/Game/GamePlay/Game/Character/MotionALSComponent_BP.Ragdoll Start` _motionalscomponent_bp :!label _label))
      (:`NewEnumerator1`
        (goto _label))
      (:`NewEnumerator2`
        (goto _label))
      (:`NewEnumerator4`
        (goto _label))
      (:`NewEnumerator3`
        (`/Game/GamePlay/Game/Character/MotionALSComponent_BP.Ragdoll End` _motionalscomponent_bp)))))

(event `self.ReceiveTick`
  (params (DeltaSeconds :type "Float (single-precision)"))
  (`parent.ReceiveTick` DeltaSeconds))

(fn `UserConstructionScript`)