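; Player character for motion matching locomotion with root motion, mouse camera control, and walk, sprint and strafe modes.
; Each tick it feeds camera-relative input to a TrajectoryGenerator, applies trajectory error warping and teleports the character back near the origin after a fall.
; Mode changes retune trajectory speed, input profile, turn response or warping, and walking also sets a "Walk" trait.
; Experimental distance-matching triggers are present but never run.
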(event `InputAction|Walk`
  (params (Key :type "Key Structure"))
  ;[1 1 1] Walking
  (:`Pressed`
    (`self.BeginWalk`))
  (:`Released`
    (`self.EndWalk`)))

(event `InputAxisKey|MouseX`
  (params (AxisValue :type "Float (single-precision)"))
  ;[1 1 1] Camera Control
  (`self.AddControllerYawInput` (* AxisValue (`self.CamSpeed_Yaw`))))

(event `InputAction|Sprint`
  (params (Key :type "Key Structure"))
  ;[1 1 1] Sprinting
  (:`Pressed`
    (`self.BeginSprint`))
  (:`Released`
    (`self.EndSprint`)))

(event `self.ReceiveBeginPlay`
  ;[1 1 1] Bind the input profile to the trajectory generator. Can be changed at runtime if required.
  (`TrajectoryGenerator_Base.SetInputProfile` (`self.TrajectoryGenerator`) (`self.InputProfile_General`))
  (`AnimInstance.SetRootMotionMode` (`SkeletalMeshComponent.GetAnimInstance` (`self.Mesh`)) "RootMotionFromEverything"))

(event `InputAxisKey|MouseY`
  (params (AxisValue :type "Float (single-precision)"))
  ;[1 1 1] Camera Control
  (`self.AddControllerPitchInput` (* AxisValue (`self.CamSpeed_Pitch`) -1.0)))

(event `InputAction|Strafe`
  (params (Key :type "Key Structure"))
  ;[1 1 1] Strafing
  (:`Pressed`
    (`self.ToggleStrafe`)))

(event `self.ReceiveTick`
  (params (DeltaSeconds :type "Float (single-precision)"))
  (bind (_returnvalue_x _returnvalue_y _returnvalue_z) (`KismetMathLibrary.BreakVector` (`self.K2_GetActorLocation`)))
  (`|ExecutionSequence`
    (:`then_0`
      ;[1 1 1] Set input vector on the trajectory generator to generate a trajectory for motion matching
      ;;[1 0.9524 0] Transform the input values with the camera so that input is relative the player's perspective
      (bind _returnvalue (`MMBlueprintFunctionLibrary.GetVectorRelativeToCamera` (`self.GetInputAxisValue`) (`self.GetInputAxisValue`) (`self.Camera`)))
      (`TrajectoryGenerator_Base.SetTrajectoryInput` (`self.TrajectoryGenerator`) (.x _returnvalue) (.y _returnvalue) 0.0)
      ;[1 1 1] Sets the strafe direction of the trjaectory generator relative to the camera
      (if (`self.IsStrafing`)
        (`TrajectoryGenerator.SetStrafeDirectionFromCamera` (`self.TrajectoryGenerator`) (`self.Camera`))))
    (:`then_1`
      ;[1 1 1] Trajectory Error Warping
      (`TrajectoryErrorWarping.ApplyTrajectoryErrorWarping` (`self.TrajectoryErrorWarping`) DeltaSeconds 1.0))
    (:`then_2`)
    (:`then_3`
      ;[1 1 1] Teleport to 0,0,0 if the character falls of the edge
      (if (< _returnvalue_z -2000.0)
        (`self.K2_SetActorLocation` (0.0 0.0 150.0) false true)))))

(fn `BeginSprint`
  (bind _trajectorygenerator (`self.TrajectoryGenerator`))
  (if (`self.IsStrafing`)
    (`self.EndStrafe`))
  (set `self.IsSprinting` true)
  (set `TrajectoryGenerator.MaxSpeed` 675.0 _trajectorygenerator)
  (`TrajectoryGenerator_Base.SetInputProfile` _trajectorygenerator (`self.InputProfile_Sprint`)))

(fn `BeginStrafe`
  (bind _trajectorygenerator (`self.TrajectoryGenerator`))
  (bind _trajectoryerrorwarping (`self.TrajectoryErrorWarping`))
  (set `self.IsStrafing` true)
  (set `TrajectoryGenerator.TrajectoryBehaviour` "Strafe" _trajectorygenerator)
  (set `TrajectoryGenerator.TurnResponse` 50.0 _trajectorygenerator)
  (set `TrajectoryErrorWarping.WarpMode` "Strafe" _trajectoryerrorwarping)
  (set `TrajectoryErrorWarping.WarpRate` 180.0 _trajectoryerrorwarping)
  (set `TrajectoryErrorWarping.ErrorActivationRange` (5.0 180.0) _trajectoryerrorwarping))

(fn `BeginWalk`
  (bind _canwalk (`self.CanWalk`))
  (if _canwalk
    (`MMBlueprintFunctionLibrary.AddTrait` "Walk" (`self.RequiredTraits`))
    (set `TrajectoryGenerator.MaxSpeed` 175.0 (`self.TrajectoryGenerator`))))

(fn `CanWalk`
  (returns (CanWalk :type Boolean))
  (if (`self.IsSprinting`)
    (return false)
    (else
      (return true))))

(fn `EndSprint`
  (bind _trajectorygenerator (`self.TrajectoryGenerator`))
  (set `self.IsSprinting` false)
  (set `TrajectoryGenerator.MaxSpeed` 400.0 _trajectorygenerator)
  (`TrajectoryGenerator_Base.SetInputProfile` _trajectorygenerator (`self.InputProfile_General`)))

(fn `EndStrafe`
  (bind _trajectorygenerator (`self.TrajectoryGenerator`))
  (bind _trajectoryerrorwarping (`self.TrajectoryErrorWarping`))
  (set `self.IsStrafing` false)
  (set `TrajectoryGenerator.TrajectoryBehaviour` "Standard" _trajectorygenerator)
  (set `TrajectoryGenerator.TurnResponse` 10.0 _trajectorygenerator)
  (set `TrajectoryErrorWarping.WarpMode` "Standard" _trajectoryerrorwarping)
  (set `TrajectoryErrorWarping.WarpRate` 60.0 _trajectoryerrorwarping)
  (set `TrajectoryErrorWarping.ErrorActivationRange` (0.25 30.0) _trajectoryerrorwarping))

(fn `EndWalk`
  (`MMBlueprintFunctionLibrary.RemoveTrait` "Walk" (`self.RequiredTraits`))
  (set `TrajectoryGenerator.MaxSpeed` 420.0 (`self.TrajectoryGenerator`)))

(fn `ToggleStrafe`
  (if (`self.IsSprinting`)
    _
    (elif (`self.IsStrafing`)
      (`self.EndStrafe`)
      (else
        (`self.BeginStrafe`)))))

(fn `UserConstructionScript`)